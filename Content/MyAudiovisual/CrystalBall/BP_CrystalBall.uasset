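; BP_CrystalBall is a crystal ball pawn that glows in a configurable color and takes MoveForward and MoveRight input along world axes, scaled by MoveSpeed.
; The construction script pushes Color to the Niagara effect and point light, sets the light intensity, and builds one dynamic material instance shared by the four swirl layers.
; BeginPlay activates the Niagara effect.
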(event EventBeginPlay
  (Components|Activation|Activate (Variables|Default|GetNiagara) false))

(event EventTick
  (params (DeltaSeconds :type Float%20%28single-precision%29)))

(event Collision|EventActorBeginOverlap
  (params (OtherActor :type Actor%20Object%20Reference)))

(event Input|AxisEvents|InputAxisMoveForward
  (params (AxisValue :type Float%20%28single-precision%29))
  (Pawn|Input|AddMovementInput (Math|Vector|MakeVector (Variables|Default|GetMoveSpeed) 0.0 0.0) AxisValue false))

(event Input|AxisEvents|InputAxisMoveRight
  (params (AxisValue :type Float%20%28single-precision%29))
  (Pawn|Input|AddMovementInput (Math|Vector|MakeVector 0.0 (Variables|Default|GetMoveSpeed) 0.0) AxisValue false))

(fn ConstructionScript
  (Niagara|SetNiagaraVariable(LinearColor) (Variables|Default|GetNiagara) "MateriaColor" (Variables|Default|GetColor))
  (Rendering|Components|Light|SetLightColor (Variables|Default|GetPointLight) (Variables|Default|GetColor) true)
  (Rendering|Components|Light|SetIntensity (Variables|Default|GetPointLight) (Variables|Default|GetLight%20Intensity))
  (bind _returnvalue (Rendering|Material|CreateDynamicMaterialInstance 0 "None" "None" :!class /Script/Engine.KismetMaterialLibrary))
  (Variables|Default|SetMID _returnvalue)
  (Rendering|Material|SetMaterial (Variables|Default|GetSwirls_Middle_Layer) 0 (Variables|Default|GetMID))
  (Rendering|Material|SetVectorParameterValue (Variables|Default|GetMID) "Color" (Variables|Default|GetColor) :!class /Script/Engine.MaterialInstanceDynamic))