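; BP_AudioSource is an audio-visual source actor whose sound and Niagara effect respond to the player's distance.
; Audio starts on BeginPlay, and Tick sets its volume higher as the player nears, using clamped, inverted range mapping.
; Tick also toggles Niagara near its maximum range and feeds it distance as radius, with velocity and alpha scaled by proximity.
; A SpawnGrid function spawns a square BP_Cube grid, but nothing here calls it.
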(event EventBeginPlay
  ;[1 1 1] Audio Effect Driven by Distance To Player
  (Audio|Components|Audio|Play (Variables|Default|GetAudio) 0.0))

(event Collision|EventActorBeginOverlap
  (params (OtherActor :type Actor%20Object%20Reference)))

(event EventTick
  (params (DeltaSeconds :type Float%20%28single-precision%29))
  (bind _returnvalue (Game|Player|GetPlayerPawn 0))
  (bind _niagara (Variables|Default|GetNiagara))
  (bind _audiorangemin (Variables|Default|GetAudioRangeMin))
  (bind _niagara_2 (Variables|Default|GetNiagara))
  (bind _particlerangemin (Variables|Default|GetParticleRangeMin))
  (bind _particlerangemax (Variables|Default|GetParticleRangeMax))
  (bind _returnvalue_2 (- _particlerangemax _particlerangemin))
  (bind _returnvalue_3 (Transformation|GetDistanceTo _returnvalue))
  (bind _returnvalue_4 (- _returnvalue_3 _particlerangemin))
  (bind _returnvalue_5 (/ _returnvalue_4 _returnvalue_2))
  (bind _returnvalue_6 (Math|Float|Clamp(Float) _returnvalue_5 0.1 0.9))
  (bind _returnvalue_7 (- 1.0 _returnvalue_6))
  (Utilities|FlowControl|Sequence
    (:then_0
      ;[1 1 1] Particle Effect Driven by Distance To Player
      (if (< _returnvalue_3 (+ (Variables|Default|GetParticleRangeMax) 2e+02))
        (Components|Activation|Activate _niagara_2 false)
        (else
          (Components|Activation|Deactivate _niagara_2))))
    (:then_1
      (Niagara|SetNiagaraVariable(Float) _niagara "User.Radius" _returnvalue_3)
      (Niagara|SetNiagaraVariable(Float) _niagara "User.VelocityScale" (* _returnvalue_7 3e+02))
      (Niagara|SetNiagaraVariable(Float) _niagara "User.Alpha" (* _returnvalue_7 1.0))
      (if (< _returnvalue_3 _particlerangemax)
        (Development|PrintString (Utilities|String|ToString(Float) _returnvalue_7) false)))
    (:then_2
      ;[1 1 1] Audio Effect Driven by Distance To Player
      (Audio|Components|Audio|SetVolumeMultiplier (Variables|Default|GetAudio) (- 1.0 (Math|Float|Clamp(Float) (/ (- _returnvalue_3 _audiorangemin) (- (Variables|Default|GetAudioRangeMax) _audiorangemin)) 0.1 0.9)) :!class /Script/Engine.AudioComponent))))

(fn ConstructionScript)

(fn SpawnGrid
  (bind _distance (Variables|Default|GetDistance))
  (for _index (range 0 (- (Variables|Default|GetCubeCount) 1))
    (bind _returnvalue (Game|SpawnActorfromClass "/Game/MyAudiovisual/BP/BP_Cube.BP_Cube_C" (Math|Transform|MakeTransform (Math|Vector|MakeVector (* (Variables|Default|GetRow) _distance) (* (Variables|Default|GetColumn) _distance) 0.0) "0, 0, 0" "1,1,1") "AlwaysSpawn" 0 0))
    (Utilities|Array|Add (Variables|Default|GetBP_CubeArray) _returnvalue)
    (Math|Integer|IncrementInt (Variables|Default|GetRow)
      (:%20%20
        (if (== (Variables|Default|GetRow) (Math|Float|Truncate (Math|Float|Sqrt (Math|Conversions|ToFloat(Integer) (Variables|Default|GetCubeCount)))))
          (Math|Integer|IncrementInt (Variables|Default|GetColumn)
            (:%20%20
              (Variables|Default|SetRow 0))))))))