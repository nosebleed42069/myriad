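; Effect actor that adds an extra particle layer to an Entity actor and damages the player through it.
; On BeginPlay it passes itself to the ExtraLayer effect as a callback object, and each tick it teleports that layer to the Entity's location.
; When particle data comes back from the effect, it applies fixed damage to the first player pawn without inspecting that data.
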(event EventBeginPlay
  (Class|NiagaraComponent|SetVariableObject (Variables|Default|GetExtraLayer) "BP_extra" self))

(event EventParticleData
  (params (Data :type Array%20of%20Basic%20Particle%20Data%20Structures) (NiagaraSystem :type Niagara%20System%20Object%20Reference))
  (Game|Damage|ApplyDamage (Game|Player|GetPlayerPawn 0) 1e+01 0 0))

(event EventTick
  (params (DeltaSeconds :type Float%20%28single-precision%29))
  (Transformation|SetWorldLocation (Variables|Default|GetExtraLayer) (Transformation|GetActorLocation (Variables|Default|Getentity)) false true))

(fn ConstructionScript)