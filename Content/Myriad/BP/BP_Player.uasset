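; BP_Player is the player's sphere, which moves along world axes and glows according to its distance from the nearest BP_AudioSource.
; The construction script creates a dynamic material on the sphere, and BeginPlay caches all audio sources.
; Each Tick finds the nearest source and maps inverted, clamped distance onto that source's emissive range, brightening the sphere as it gets closer.
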(event EventBeginPlay
  (bind _outactors (Actor|GetAllActorsOfClass "/Game/Myriad/BP/BP_AudioSource.BP_AudioSource_C"))
  (Variables|Default|SetOut%20Actors _outactors))

(event Collision|EventActorBeginOverlap
  (params (OtherActor :type Actor%20Object%20Reference)))

(event EventTick
  (params (DeltaSeconds :type Float%20%28single-precision%29))
  (bind _returnvalue (Transformation|GetActorLocation))
  (bind _out_actors (Variables|Default|GetOut%20Actors))
  (bind (_distance _returnvalue_2) (Actor|FindNearestActor _returnvalue _out_actors))
  (bind _asbp_audio_source (Utilities|Casting|CastToBP_AudioSource _returnvalue_2))
  (Rendering|Material|SetScalarParameterValue (Variables|Default|GetDynamicMat) "Emissive Multiplier" (Math|Float|MapRangeClamped (- 1.0 (Math|Float|Clamp(Float) (/ (- _distance (Variables|/Game/Myriad/BP/BP_AudioSource.BP_AudioSource_C|GetEmissiveRangeMin _asbp_audio_source)) (- (Variables|/Game/Myriad/BP/BP_AudioSource.BP_AudioSource_C|GetEmissiveRangeMax _asbp_audio_source) (Variables|/Game/Myriad/BP/BP_AudioSource.BP_AudioSource_C|GetEmissiveRangeMin _asbp_audio_source))) 0.1 0.9)) 0.1 0.9 (Variables|/Game/Myriad/BP/BP_AudioSource.BP_AudioSource_C|GetEmissiveMin _asbp_audio_source) (Variables|/Game/Myriad/BP/BP_AudioSource.BP_AudioSource_C|GetEmissiveMax _asbp_audio_source)) :!class /Script/Engine.MaterialInstanceDynamic))

(event Input|AxisEvents|InputAxisMoveForward
  (params (AxisValue :type Float%20%28single-precision%29))
  (Pawn|Input|AddMovementInput (Math|Vector|MakeVector (Variables|Default|GetMoveSpeed) 0.0 0.0) AxisValue false))

(event Input|AxisEvents|InputAxisMoveRight
  (params (AxisValue :type Float%20%28single-precision%29))
  (Pawn|Input|AddMovementInput (Math|Vector|MakeVector 0.0 (Variables|Default|GetMoveSpeed) 0.0) AxisValue false))

(fn ConstructionScript
  (bind _returnvalue (Rendering|Material|CreateDynamicMaterialInstance (Variables|Default|GetSphere) 0 (Variables|Default|GetSourceMaterial) "None" :!class /Script/Engine.PrimitiveComponent))
  (Variables|Default|SetDynamicMat _returnvalue))