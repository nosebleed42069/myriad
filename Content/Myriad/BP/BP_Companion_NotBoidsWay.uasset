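; Companion actor that trails a Target actor by moving directly toward it, without boids steering.
; Each Tick it starts a MoveComponentTo on the root toward Target's location, with a duration that shortens as the player's distance grows between DistanceMin and DistanceMax.
; Its mesh turns billboard-like to face the player.
; It also prints the computed duration every frame as debug output.
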(event EventBeginPlay)

(event Collision|EventActorBeginOverlap
  (params (OtherActor :type Actor%20Object%20Reference)))

(event EventTick
  (params (DeltaSeconds :type Float%20%28single-precision%29))
  (bind _returnvalue (Transformation|GetActorLocation))
  (bind _returnvalue_2 (Game|Player|GetPlayerPawn 0))
  (bind _distancemin (Variables|Default|GetDistanceMin))
  (bind _distancemax (Variables|Default|GetDistanceMax))
  (bind _returnvalue_3 (- _distancemax _distancemin))
  (bind _returnvalue_4 (Transformation|GetActorLocation _returnvalue_2))
  (bind _returnvalue_5 (- _returnvalue_4 _returnvalue))
  (bind _returnvalue_6 (Math|Vector|VectorLength _returnvalue_5))
  (bind _returnvalue_7 (- _returnvalue_6 _distancemin))
  (bind _returnvalue_8 (/ _returnvalue_7 _returnvalue_3))
  (bind _returnvalue_9 (Math|Float|Clamp(Float) _returnvalue_8))
  (bind _returnvalue_10 (Math|Float|MapRangeClamped _returnvalue_9 0.0 1.0 5.0 2.0))
  (Utilities|FlowControl|Sequence
    (:then_0
      (Components|MoveComponentTo (Variables|Transformation|GetRootComponent) (Transformation|GetActorLocation (Variables|Default|GetTarget)) "0, 0, 0" false false _returnvalue_10 false))
    (:then_1
      ;[1 1 1] Actor always looks at the palyer (Similar to Billboard)
      (Transformation|SetRelativeRotation (Variables|Default|GetStaticMesh) (Math|Rotator|FindLookatRotation (Transformation|GetActorLocation) (Transformation|GetActorLocation (Game|Player|GetPlayerPawn 0))) false false))
    (:then_2
      (Development|PrintString (Utilities|String|ToString(Float) _returnvalue_10)))))

(fn ConstructionScript)