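; Player-controlled crystal ball that moves on axis input and wins over boid companions by matching their pulse rhythm with the space bar.
; Overlapping an immobile companion enters connection mode, and each press flashes a light, triggers Niagara and records the interval since the previous press.
; Tick animates a sine glow on the core material and frees the companion once the last three intervals approximate its PulseInterval.
; Damage briefly disables collision.
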(event OnComponentBeginOverlap(CompanionTrigger)
  (params (OverlappedComponent :type Primitive%20Component%20Object%20Reference) (OtherActor :type Actor%20Object%20Reference) (OtherComp :type Primitive%20Component%20Object%20Reference) (OtherBodyIndex :type Integer) (bFromSweep :type Boolean) (SweepResult :type Hit%20Result%20Structure%20%28by%20ref%29))
  ;[1 0.5432 0.1131] Detect Companion in range and respond
  (bind _asbp_boids_companion (Utilities|Casting|CastToBP_Boids_Companion OtherActor))
  (if (not (Variables|/Game/Myriad/Companions/BP_Boids_Companion.BP_Boids_Companion_C|GetcanMove _asbp_boids_companion))
    (CallFunction|EnterConnectionMode _asbp_boids_companion)))

(event OnComponentEndOverlap(CompanionTrigger)
  (params (OverlappedComponent :type Primitive%20Component%20Object%20Reference) (OtherActor :type Actor%20Object%20Reference) (OtherComp :type Primitive%20Component%20Object%20Reference) (OtherBodyIndex :type Integer))
  ;[1 0.5432 0.1131] Detect Companion in range and respond
  (bind _asbp_boids_companion (Utilities|Casting|CastToBP_Boids_Companion OtherActor))
  (if (not (Variables|/Game/Myriad/Companions/BP_Boids_Companion.BP_Boids_Companion_C|GetcanMove _asbp_boids_companion))
    (CallFunction|ExitConnectionMode)
    (Development|PrintString "exit")))

(event Game|Damage|EventAnyDamage
  (params (Damage :type Float%20%28single-precision%29) (DamageType :type Damage%20Type%20Object%20Reference) (InstigatedBy :type Controller%20Object%20Reference) (DamageCauser :type Actor%20Object%20Reference))
  ;[1 0.003331 0] Process Damage
  (Development|PrintString (Utilities|String|ToString(Float) Damage))
  (Collision|SetActorEnableCollision false)
  (Utilities|FlowControl|Delay 1.0)
  (Collision|SetActorEnableCollision true))

(event EventTick
  (params (DeltaSeconds :type Float%20%28single-precision%29))
  (Utilities|FlowControl|Sequence
    (:then_0
      (CallFunction|MaintainPulsing DeltaSeconds)
      ;[0.384 0.5817 1] Apply Pulsing to the core material
      (Rendering|Material|SetScalarParameterValue (Variables|Default|GetDynamicMat) "Core Brightness" (CallFunction|CalculatePulsingFrequence) :!class /Script/Engine.MaterialInstanceDynamic))
    (:then_1
      ;[1 0.9882 0] Compare last 3 values in TImeDeltas array with companion's pulsing
      (if (Variables|Default|GetplayerIsInConnectionMode)
        ;[0.4113 1 0] Attach companion and exit the connection mode
        (if (Math|Boolean|ANDBoolean (CallFunction|GetElementbyIndex 0.5) (CallFunction|GetElementbyIndex 0.5 1) (CallFunction|GetElementbyIndex 0.5 2))
          (Variables|/Game/Myriad/Companions/BP_Boids_Companion.BP_Boids_Companion_C|SetcanMove (Variables|Default|Getcompanion) true)
          (CallFunction|ExitConnectionMode))))))

(event Input|AxisEvents|InputAxisMoveForward
  (params (AxisValue :type Float%20%28single-precision%29))
  ;[1 0.1249 0.8899] Character Movement
  (Pawn|Input|AddMovementInput (Math|Vector|MakeVector (Variables|Default|GetMoveSpeed) 0.0 0.0) AxisValue false))

(event Input|AxisEvents|InputAxisMoveRight
  (params (AxisValue :type Float%20%28single-precision%29))
  ;[1 0.1249 0.8899] Character Movement
  (Pawn|Input|AddMovementInput (Math|Vector|MakeVector 0.0 (Variables|Default|GetMoveSpeed) 0.0) AxisValue false))

(event Input|KeyboardEvents|SpaceBar
  (params (Key :type Key%20Structure :default "None"))
  ;[1 1 1] Unused elements
)

(event Input|KeyboardEvents|SpaceBar
  (params (Key :type Key%20Structure :default "None"))
  ;[0.176 0.03149 0.04588] ProcessInputToGetTImeFrames
  (:Pressed
    (Utilities|ApplyPulseEffect)
    (if (== (Utilities|Array|Length (Variables|Pulsing|GetTimeframes)) 0)
      (CallFunction|AppendArray)
      (else
        (CallFunction|AppendArray)
        ;[0.4277 1 0.2419 1 24] SetTImeDeltasBetweenTimeFrames
        (Utilities|Array|SetArrayElem (Variables|Pulsing|GetTimeDeltas) (Variables|Pulsing|GetnumberOfInputs) (CallFunction|CalculateTimeDelta) true)))))

(event Input|KeyboardEvents|SpaceBar
  (params (Key :type Key%20Structure :default "None"))
  (:Pressed
    (Components|Activation|Activate (Variables|Default|GetNiagaraPlayerPulsing) false)))

(fn ConstructionScript
  (Utilities|FlowControl|Sequence
    (:then_0
      (Niagara|SetNiagaraVariable(LinearColor) (Variables|Default|GetNiagara) "MateriaColor" (Variables|Default|GetColor))
      (Rendering|Components|Light|SetLightColor (Variables|Default|GetPointLight) (Variables|Default|GetColor) true)
      (Rendering|Components|Light|SetIntensity (Variables|Default|GetPointLight) (Variables|Default|GetLight%20Intensity)))
    (:then_1
      (bind _returnvalue (Rendering|Material|CreateDynamicMaterialInstance (Variables|Default|GetCore) 0 (Variables|Default|GetSourceMaterial) "None" :!class /Script/Engine.PrimitiveComponent))
      (Variables|Default|SetDynamicMat _returnvalue))
    (:then_2
      (Niagara|SetNiagaraVariable(LinearColor) (Variables|Default|GetNiagaraPlayerPulsing) "MaterialColor" (Variables|Default|GetColor)))))

(fn NewFunction0
  (params (Value :type Integer%20%28by%20ref%29))
  (Math|Integer|IncrementInt Value))

(fn ProcessInput
  (Variables|Pulsing|SetnumberOfInputs (+ (Variables|Pulsing|GetnumberOfInputs) 1))
  (if (== (Variables|Pulsing|GetnumberOfInputs) 2)
    _))

(fn GetElementbyIndex
  (params (ErrorTolerance :type Float%20%28single-precision%29) (Index :type Integer))
  (bind _timedeltas (Variables|Pulsing|GetTimeDeltas))
  (return (Math|Float|NearlyEqual(Float) (Utilities|Array|Get(acopy) _timedeltas (- (Utilities|Array|LastIndex _timedeltas) Index)) (Variables|/Game/Myriad/Companions/BP_Boids_Companion.BP_Boids_Companion_C|GetPulseInterval (Variables|Default|Getcompanion)) ErrorTolerance)))

(fn AppendArray
  (Utilities|Array|SetArrayElem (Variables|Pulsing|GetTimeframes) (Variables|Pulsing|GetnumberOfInputs) (Utilities|Time|GetGameTimeinSeconds) true)
  (Variables|Pulsing|SetnumberOfInputs (+ (Variables|Pulsing|GetnumberOfInputs) 1)))

(fn CalculateTimeDelta
  (return (- (Utilities|Array|Get(acopy) (Variables|Pulsing|GetTimeframes) (Utilities|Array|LastIndex (Variables|Pulsing|GetTimeframes))) (Utilities|Array|Get(acopy) (Variables|Pulsing|GetTimeframes) (- (Utilities|Array|LastIndex (Variables|Pulsing|GetTimeframes)) 1)))))

(fn CalculatePulsingFrequence
  (return (+ (* (Math|Trig|Sin(Radians) (* (Math|Float|%(Float) (Variables|Default|GetTimer) (* (Math|Trig|GetPI) 2.0)) (+ (Variables|Default|GetPulsingInitialSpeed) (Variables|Default|GetIncreasingValue)))) 0.1) 0.1)))

(fn MaintainPulsing
  (params (DeltaTime :type Float%20%28single-precision%29))
  (bind _output_get (Variables|Default|SetDeltaTime DeltaTime))
  (Variables|Default|SetTimer (+ (Variables|Default|GetTimer) _output_get))
  (bind _output_get_2 (Variables|Default|SetIncreasingValue (- (Variables|Default|GetIncreasingValue) (* 0.0 (Variables|Default|GetDeltaTime)))))
  (if (<= _output_get_2 0.0)
    (Variables|Default|SetIncreasingValue 0.0)))

(fn EnterConnectionMode
  (params (companion :type BP%20Boids%20Companion%20Object%20Reference))
  (Variables|Default|Setcompanion companion)
  (Variables|Default|SetplayerIsInConnectionMode true)
  (Utilities|Array|Clear (Variables|Pulsing|GetTimeframes))
  (Utilities|Array|Clear (Variables|Pulsing|GetTimeDeltas)))

(fn ExitConnectionMode
  (Variables|Default|SetplayerIsInConnectionMode false)
  (Utilities|Array|Clear (Variables|Pulsing|GetTimeframes))
  (Utilities|Array|Clear (Variables|Pulsing|GetTimeDeltas)))