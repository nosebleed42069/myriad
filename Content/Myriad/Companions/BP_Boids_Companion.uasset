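; Flocking companion actor with a randomly picked look (star, fish, insect or crystal) that pulses and reacts with Niagara particles as the player nears.
; Once movable, its physics mesh flies forward at distance-scaled speed, using cross-product angular velocity to home in on a random offset around the player.
; When detached, it homes on the crystal ball's EntityToFight instead.
; Tick also drives glow, trail and color blending toward the player's color.
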(event EventTick
  (params (DeltaSeconds :type Float%20%28single-precision%29))
  (bind _returnvalue (Game|Player|GetPlayerPawn 0))
  (bind _dynamicmat (Variables|Default|GetDynamicMat))
  (bind _niagara (Variables|Default|GetNiagara))
  (bind _niagara_2 (Variables|Default|GetNiagara))
  (bind _pulselight (Variables|Default|GetPulseLight))
  (bind _emissive (Variables|Default|GetEmissive))
  (bind _returnvalue_2 (Transformation|GetDistanceTo _returnvalue))
  (Utilities|FlowControl|Sequence
    (:then_0
      ;[1 0.7645 0] Home-in to the player's approximate position
      (if (Variables|Default|GetcanMove)
        (Physics|SetPhysicsLinearVelocity (Variables|Default|GetMesh) (CallFunction|GetForvardVelocityVector) false "None")
        (if (Variables|Default|GetisAttachedToPlayer)
          (Class|PrimitiveComponent|SetPhysicsAngularVelocityinRadians (Variables|Default|GetMesh) (CallFunction|ApplyCrossProduct (Transformation|GetActorLocation (Game|Player|GetPlayerPawn 0)) (Variables|Default|GetTargetLocationOffset)) false "None")
          (else
            ;[1 0.2093 0.1476] if player damamged, attach component to the current entity
            (bind _asbp_crystal_ball (Utilities|Casting|CastToBP_CrystalBall (Game|Player|GetPlayerPawn 0)))
            (Variables|Default|SetentityAttachTo (Variables|/Game/Myriad/CrystalBall/BP_CrystalBall.BP_CrystalBall_C|GetEntityToFight _asbp_crystal_ball))
            (Class|PrimitiveComponent|SetPhysicsAngularVelocityinRadians (Variables|Default|GetMesh) (CallFunction|ApplyCrossProduct (Transformation|GetActorLocation (Variables|Default|GetentityAttachTo)) "0, 0, 0") false "None")))))
    (:then_1
      ;[1 1 1] Apply light pulse
      (if (Utilities|Enum|NotEqual(Enum) (Utilities|GetObjectName (stale EventBeginPlay _output_get)) "M_CompanionCrystal_Inst")
        (Rendering|SetVisibility _pulselight (Variables|Default|GetisVisible) false)
        (Rendering|Components|Light|SetLightColor _pulselight (Variables|Default|GetColor) true)
        (elif (Variables|Default|GetSetElpisParticles)
          (Components|Activation|Activate (Variables|Default|GetNS_FirstCompanionPulse_01) false)
          (Variables|Default|SetSetElpisParticles false)
          (Utilities|FlowControl|Delay 0.2)
          (Components|Activation|Deactivate (Variables|Default|GetNS_FirstCompanionPulse_01))
          (Utilities|FlowControl|Delay (- (Variables|Default|GetPulseInterval) 0.2))
          (Variables|Default|SetSetElpisParticles true))))
    (:then_2
      ;[1 1 1] Guiding
      (Variables|Default|SetisGuiding (< _returnvalue_2 (Variables|Default|GetguidingRange)))
      ;;[1 1 1] CompanionTrigger Radius
      (bind _output_get (Variables|Default|SetisGreeting (<= _returnvalue_2 (Variables|Default|GetgreetingRange))))
      (Niagara|SetNiagaraVariable(Float) _niagara_2 "User.Radius" _returnvalue_2)
      (if _output_get
        (Niagara|SetNiagaraVariable(Float) _niagara_2 "User.SpawnGuiding" 1.0)
        (else
          (Niagara|SetNiagaraVariable(Float) _niagara_2 "User.SpawnGuiding" 0.0))))
    (:then_3
      ;[1 1 1] Greeting
      (if (Variables|Default|GetisGreeting)
        (Niagara|SetNiagaraVariable(Float) _niagara "User.AttractionStrength" 6e+01)
        (Niagara|SetNiagaraVariable(Vector3) _niagara "User.PlayerLoc" (- (Transformation|GetWorldLocation (Variables|/Script/Engine.Actor|GetRootComponent (Game|Player|GetPlayerPawn 0))) (Transformation|GetActorLocation)))
        (else
          (Niagara|SetNiagaraVariable(Float) _niagara "User.AttractionStrength" 0.0))))
    (:then_4
      ;[1 1 1] Comment
      (Niagara|SetNiagaraVariable(LinearColor) (Variables|Default|GetNiagara) "User.MyColor" (Variables|Default|GetColor))
      (Niagara|SetNiagaraVariable(LinearColor) (Variables|Default|GetNiagaraTrail) "User.MyColor" (Variables|Default|GetColor))
      (Rendering|Material|SetVectorParameterValue (Variables|Default|GetDynamicMat) "Color" (Variables|Default|GetColor) :!class /Script/Engine.MaterialInstanceDynamic))
    (:then_5
      ;[1 1 1] Sync Effect
      (if (and (Variables|Default|GetisVisible) (Variables|Default|GetisGreeting))
        (Rendering|Material|SetScalarParameterValue _dynamicmat "Emissive Multiplier" _emissive :!class /Script/Engine.MaterialInstanceDynamic)
        (else
          (Rendering|Material|SetScalarParameterValue _dynamicmat "Emissive Multiplier" 0.2 :!class /Script/Engine.MaterialInstanceDynamic))))
    (:then_6
      ;[1 1 1] Connecting
      (if (Variables|Default|GetreadyToMove)
        (Components|Activation|Deactivate (Variables|Default|GetNiagara))
        (Rendering|Material|SetScalarParameterValue _dynamicmat "Emissive Multiplier" _emissive :!class /Script/Engine.MaterialInstanceDynamic)
        (Niagara|SetNiagaraVariable(Float) (Variables|Default|GetNiagaraTrail) "User.SpawnTrail" 1.0)
        (Rendering|Material|SetScalarParameterValue (Variables|Default|GetDynamicMat) "PlayRate" 1.0 :!class /Script/Engine.MaterialInstanceDynamic)))
    (:then_7
      (if (Variables|Default|GetcanMove)
        (if (Variables|Default|GetCompanionBecomesPlayerColor)
          (Variables|Default|SetIncreaseAlpha (+ (Variables|Default|GetIncreaseAlpha) 0.001))
          (Variables|Default|SetColor (Math|Color|Lerp(LinearColor) (Variables|Default|GetColor) (Variables|/Game/Myriad/CrystalBall/BP_CrystalBall.BP_CrystalBall_C|GetColor (Variables|Default|GetPlayer)) (+ (Variables|Default|GetIncreaseAlpha) 0.001)))
          (Utilities|FlowControl|Delay 1.0)
          (Variables|Default|SetCompanionBecomesPlayerColor false))))
    (:then_8
      (if (not (Variables|Default|GetCompanionBecomesPlayerColor))
        (Variables|Default|SetColor (Variables|/Game/Myriad/CrystalBall/BP_CrystalBall.BP_CrystalBall_C|GetColor (Variables|Default|GetPlayer)))))
    (:then_9
      (Variables|Default|SetMove%20Speed (Math|Float|Lerp 1e+01 (Variables|Default|GetmaxMoveSpeed) (Math|Float|NormalizetoRange (Math|Vector|Distance(Vector) (Transformation|GetActorLocation self) (Transformation|GetActorLocation (Variables|Default|GetPlayer))) 0.0 1.2e+03))))))

(event EventBeginPlay
  (bind _flockouterbound (Variables|Default|GetFlockOuterBound))
  (bind _mesh (Variables|Default|GetMesh))
  (bind _flockinnerbound (Variables|Default|GetFlockInnerBound))
  (bind _niagara (Variables|Default|GetNiagara))
  (bind _returnvalue (* _flockouterbound -1.0))
  (bind _returnvalue_2 (* _flockinnerbound -1.0))
  (Utilities|FlowControl|Sequence
    (:then_0
      ;[0.0784 0.5759 1] Set companion in pulsing mode
      (Physics|SetSimulatePhysics (Variables|Default|GetMesh) true)
      (Variables|Default|SetPulseInterval (Math|Random|RandomFloatinRange (Variables|Default|GetminPulse) (Variables|Default|GetmaxPulse)))
      (Utilities|MaintainPulsing :!label _label)
      (goto _label))
    (:then_1
      (if (Utilities|Enum|NotEqual(Enum) (Utilities|GetObjectName (stale _output_get)) "M_CompanionCrystal_Inst")
        (Variables|Default|SetColor (Utilities|Struct|MakeLinearColor (Math|Random|RandomFloat) (Math|Random|RandomFloat) (Math|Random|RandomFloat) 1.0))))
    (:then_2
      (bind _returnvalue_3 (Actor|GetActorOfClass "/Game/Myriad/CrystalBall/BP_CrystalBall.BP_CrystalBall_C"))
      (Variables|Default|SetPlayer _returnvalue_3))
    (:then_4
      (Variables|Default|SetTargetLocationOffset (Math|Vector|MakeVector (Math|Float|SelectFloat (Math|Random|RandomFloatinRange _returnvalue _flockouterbound) (Math|Float|SelectFloat (Math|Random|RandomFloatinRange _returnvalue _returnvalue_2) (Math|Random|RandomFloatinRange _flockinnerbound _flockouterbound) (Math|Random|RandomBool)) (Math|Random|RandomBoolwithWeight 0.6)) (Math|Float|SelectFloat (Math|Float|SelectFloat (Math|Random|RandomFloatinRange _returnvalue _returnvalue_2) (Math|Random|RandomFloatinRange _flockinnerbound _flockouterbound) (Math|Random|RandomBool)) (Math|Float|SelectFloat (Math|Random|RandomFloatinRange _returnvalue_2 _flockinnerbound) (Math|Random|RandomFloatinRange _returnvalue_2 _flockinnerbound) (Math|Random|RandomBool)) (Math|Random|RandomBoolwithWeight 0.6)) 0.0)))
    (:then_5
      (bind _output_get (Variables|Default|SetSource%20Material self (.OutItem (Utilities|Array|Random (Variables|Default|GetSourceMaterialArray)))))
      (Development|PrintString (Utilities|GetObjectName _output_get))
      (if (Utilities|Enum|Equal(Enum) (Utilities|GetObjectName _output_get) "MI_Star")
        (Components|StaticMesh|SetStaticMesh (Variables|Default|GetMesh) "/Game/Myriad/Companions/SM_Star.SM_Star")
        (Variables|Default|SetNew%20Mesh "/Game/Myriad/Companions/SM_Star.SM_Star")
        (elif (Utilities|Enum|Equal(Enum) (Utilities|GetObjectName _output_get) "MI_Fish")
          (Components|StaticMesh|SetStaticMesh (Variables|Default|GetMesh) "/Game/Myriad/Companions/SM_Fish.SM_Fish")
          (Variables|Default|SetNew%20Mesh "/Game/Myriad/Companions/SM_Fish.SM_Fish")
          (elif (Utilities|Enum|Equal(Enum) (Utilities|GetObjectName _output_get) "MI_Flydragon")
            (Components|StaticMesh|SetStaticMesh (Variables|Default|GetMesh) "/Game/Myriad/Companions/SM_Insect_01.SM_Insect_01")
            (Variables|Default|SetNew%20Mesh "/Game/Myriad/Companions/SM_Insect_01.SM_Insect_01")
            (elif (Utilities|Enum|Equal(Enum) (Utilities|GetObjectName _output_get) "M_CompanionCrystal_Inst")
              (Components|StaticMesh|SetStaticMesh (Variables|Default|GetMesh) "/Game/Myriad/Companions/SM_Pyramid.SM_Pyramid")
              (Variables|Default|SetSource%20Material (Variables|Default|GetSource%20Material))
              (Variables|Default|SetTargetLocationOffset "300.000000,300.000000,0.000000"))))))
    (:then_6
      (Components|StaticMesh|SetStaticMesh _mesh (Variables|Default|GetNew%20Mesh))
      (bind _returnvalue_4 (Rendering|Material|CreateDynamicMaterialInstance _mesh 0 (Variables|Default|GetSource%20Material) "None" :!class /Script/Engine.PrimitiveComponent))
      (bind _output_get_2 (Variables|Default|SetDynamicMat _returnvalue_4))
      (Rendering|Material|SetVectorParameterValue _output_get_2 "Color" (Variables|Default|GetColor) :!class /Script/Engine.MaterialInstanceDynamic))
    (:then_7
      ;[1 1 1] Comment
      (Components|Activation|Activate _niagara false)
      (Niagara|SetNiagaraVariable(Float) _niagara "User.AttractionStrength" 0.0)
      (Niagara|SetNiagaraVariable(Float) _niagara "User.SpawnGuiding" 0.0)
      (Rendering|Material|SetScalarParameterValue (Variables|Default|GetDynamicMat) "Emissive Multiplier" 0.5 :!class /Script/Engine.MaterialInstanceDynamic)
      (Rendering|Material|SetScalarParameterValue (Variables|Default|GetDynamicMat) "PlayRate" 0.0 :!class /Script/Engine.MaterialInstanceDynamic))))

(fn ConstructionScript)

(fn ApplyCrossProduct
  (params (TargetPos :type Vector) (posApproximation :type Vector))
  (return (* (Math|Vector|CrossProduct (Math|Vector|Normalize (- (+ TargetPos posApproximation) (Transformation|GetWorldLocation (Variables|Default|GetMesh)))) (* (Math|Vector|GetForwardVector (Variables|Default|GetMesh)) "1.000000,20.000000,1.000000")) -1.0)))

(fn GetForwardStartandEndPoints
  (params (Mesh :type Static%20Mesh%20Component%20Object%20Reference) (StartPointMultiplier :type Float%20%28single-precision%29))
  (bind _returnvalue (Transformation|GetWorldLocation Mesh))
  (return _returnvalue (+ _returnvalue (* (Math|Vector|GetForwardVector Mesh) StartPointMultiplier))))

(fn GetForvardVelocityVector
  (return (* (Math|Vector|GetForwardVector (Variables|Default|GetMesh)) (Variables|Default|GetMove%20Speed))))