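; Environment actor that evolves the terrain, effects and sky with the player's companion count and the Entity's health.
; Tick feeds player position to a dynamic terrain material, and timelines blend seaweed, coral and gem layers in or out as companions change.
; Niagara lightning switches to a player-targeted beam while the Entity pulses.
; Entity death triggers one-shot timelines that reveal terrain, scale smoke, stream in MapSky and fade in sky, clouds and companions.
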(event EventBeginPlay
  (bind _dynamicmatterrain (Variables|Default|GetDynamicMatTerrain))
  (Utilities|FlowControl|Sequence
    (:then_0
      (Rendering|Material|SetScalarParameterValue _dynamicmatterrain "AmountSeaweed" 0.0 :!class /Script/Engine.MaterialInstanceDynamic)
      (Rendering|Material|SetScalarParameterValue _dynamicmatterrain "AmountCoral" 0.0 :!class /Script/Engine.MaterialInstanceDynamic)
      (Rendering|Material|SetScalarParameterValue _dynamicmatterrain "AmountGem" 0.0 :!class /Script/Engine.MaterialInstanceDynamic)
      (Rendering|Material|SetScalarParameterValue _dynamicmatterrain "PlayerAreaRadius" (Variables|Default|GetPlayerAreaRadius) :!class /Script/Engine.MaterialInstanceDynamic)
      (Rendering|Material|SetScalarParameterValue _dynamicmatterrain "OpacityRadius" 0.0 :!class /Script/Engine.MaterialInstanceDynamic)
      (Components|Activation|Deactivate (Variables|Default|GetNS_CompaionGroup)))
    (:then_1
      (Rendering|Material|SetScalarParameterValue "/Game/Myriad/Materials/MPC/MPC_Sky.MPC_Sky" "OpacitySky" 0.0 :!class /Script/Engine.KismetMaterialLibrary)
      (Rendering|Material|SetScalarParameterValue "/Game/Myriad/Materials/MPC/MPC_Sky.MPC_Sky" "OpacityCloud" 0.0 :!class /Script/Engine.KismetMaterialLibrary))))

(event Collision|EventActorBeginOverlap
  (params (OtherActor :type Actor%20Object%20Reference)))

(event EventTick
  (params (DeltaSeconds :type Float%20%28single-precision%29))
  (bind _niagaralightning (Variables|Default|GetNiagaraLightning))
  (bind _timelineblendseaweed (Variables|Default|GetTimelineBlendSeaweed))
  (bind _timelineblendcoral (Variables|Default|GetTimelineBlendCoral))
  (bind _terrainblendspeed (Variables|Default|GetTerrainBlendSpeed))
  (bind _timelineblendgem (Variables|Default|GetTimelineBlendGem))
  (bind _player (Variables|Default|GetPlayer))
  (bind _dynamicmatterrain (Variables|Default|GetDynamicMatTerrain))
  (bind _companioncounter (Variables|/Game/Myriad/CrystalBall/BP_CrystalBall.BP_CrystalBall_C|GetCompanionCounter _player))
  (Utilities|FlowControl|Sequence
    (:then_0
      (Rendering|Material|SetVectorParameterValue (Variables|Default|GetDynamicMatTerrain) "PlayerPos" (Math|Conversions|ToLinearColor(Vector) (Transformation|GetWorldLocation (Variables|/Script/Engine.Actor|GetRootComponent (Variables|Default|GetPlayer)))) :!class /Script/Engine.MaterialInstanceDynamic))
    (:then_1
      (if (and (== _companioncounter 1) (Variables|/Game/Myriad/CrystalBall/BP_CrystalBall.BP_CrystalBall_C|GetIsIncreasing _player))
        (Components|Timeline|SetPlayRate _timelineblendseaweed _terrainblendspeed)
        (bind _blendamount (Timeline|TimelineBlendSeaweed Play)
          (:Update
            (Rendering|Material|SetScalarParameterValue (Variables|Default|GetDynamicMatTerrain) "AmountSeaweed" (* _blendamount 1.0) :!class /Script/Engine.MaterialInstanceDynamic)))))
    (:then_2
      (if (and (== _companioncounter 0) (Variables|/Game/Myriad/CrystalBall/BP_CrystalBall.BP_CrystalBall_C|GetIsDecreasing _player))
        (Components|Timeline|SetPlayRate _timelineblendseaweed _terrainblendspeed)
        (Timeline|TimelineBlendSeaweed Reverse)))
    (:then_3
      (if (and (== _companioncounter 2) (Variables|/Game/Myriad/CrystalBall/BP_CrystalBall.BP_CrystalBall_C|GetIsIncreasing _player))
        (Components|Timeline|SetPlayRate _timelineblendcoral _terrainblendspeed)
        (bind _blendamount_2 (Timeline|TimelineBlendCoral Play)
          (:Update
            (Rendering|Material|SetScalarParameterValue _dynamicmatterrain "AmountCoral" (* _blendamount_2 0.75) :!class /Script/Engine.MaterialInstanceDynamic)))))
    (:then_4
      (if (and (== _companioncounter 1) (Variables|/Game/Myriad/CrystalBall/BP_CrystalBall.BP_CrystalBall_C|GetIsDecreasing _player))
        (Components|Timeline|SetPlayRate _timelineblendcoral _terrainblendspeed)
        (Timeline|TimelineBlendCoral Reverse)))
    (:then_5
      (if (and (== _companioncounter 3) (Variables|/Game/Myriad/CrystalBall/BP_CrystalBall.BP_CrystalBall_C|GetIsIncreasing _player))
        (Components|Timeline|SetPlayRate _timelineblendgem _terrainblendspeed)
        (bind _blendamount_3 (Timeline|TimelineBlendGem Play)
          (:Update
            (Rendering|Material|SetScalarParameterValue _dynamicmatterrain "AmountGem" (* _blendamount_3 1.0) :!class /Script/Engine.MaterialInstanceDynamic)))))
    (:then_6
      (if (and (== _companioncounter 2) (Variables|/Game/Myriad/CrystalBall/BP_CrystalBall.BP_CrystalBall_C|GetIsDecreasing _player))
        (Components|Timeline|SetPlayRate _timelineblendgem _terrainblendspeed)
        (Timeline|TimelineBlendGem Reverse)))
    (:then_7
      (if (<= (Variables|/Game/Myriad/BP/BP_AudioSource.BP_AudioSource_C|GetentityHealth (Variables|Default|GetEntity)) 0)
        (Utilities|FlowControl|Delay 0.2)
        (Utilities|FlowControl|Sequence
          (:then_0
            (Utilities|FlowControl|DoOnce false
              (:Completed
                (Components|Activation|Deactivate (Variables|Default|GetNiagaraLightning))
                (Components|Timeline|SetPlayRate (Variables|Default|GetTimelineTerrain) 0.2)
                (bind _opacityamount (Timeline|TimelineTerrain Play)
                  (:Update
                    (Rendering|Material|SetScalarParameterValue (Variables|Default|GetDynamicMatTerrain) "OpacityRadius" (* _opacityamount 1.0) :!class /Script/Engine.MaterialInstanceDynamic)
                    (Niagara|SetNiagaraVariable(Float) (Variables|Default|GetNiagaraSmoke) "User.MyLerp" _opacityamount)
                    (Transformation|SetRelativeScale3D (Variables|Default|GetNiagaraSmoke) (Math|Conversions|ToVector(Float) (+ (* _opacityamount 2.0) 1.0))))))))
          (:then_1
            (Utilities|FlowControl|DoOnce false
              (:Completed
                (Utilities|FlowControl|Delay 0.0)
                (Game|LoadStreamLevel(byName) "MapSky" true true)
                (Components|Timeline|SetPlayRate (Variables|Default|GetTimelineSky) 1.5)
                (bind _curve (Timeline|TimelineSky Play)
                  (:Update
                    (Rendering|Material|SetScalarParameterValue "/Game/Myriad/Materials/MPC/MPC_Sky.MPC_Sky" "OpacitySky" _curve :!class /Script/Engine.KismetMaterialLibrary)
                    (Utilities|FlowControl|Delay 0.0)
                    (Components|Timeline|SetPlayRate (Variables|Default|GetTimelineCloud) 0.35)
                    (bind _curve_2 (Timeline|TimelineCloud Play)
                      (:Update
                        (Rendering|Material|SetScalarParameterValue "/Game/Myriad/Materials/MPC/MPC_Sky.MPC_Sky" "OpacityCloud" _curve_2 :!class /Script/Engine.KismetMaterialLibrary))))))))
          (:then_2
            (Utilities|FlowControl|DoOnce false
              (:Completed
                (Utilities|FlowControl|Delay 1.0)
                (Components|Activation|Activate (Variables|Default|GetNS_CompaionGroup) false)
                (Components|Timeline|SetPlayRate (Variables|Default|GetTimeline_0) 0.25)
                (bind _curve_3 (Timeline|Timeline_0 Play)
                  (:Update
                    (Rendering|Material|SetScalarParameterValue "/Game/Myriad/Materials/MPC/MPC_Sky.MPC_Sky" "OpacityCompanions" _curve_3 :!class /Script/Engine.KismetMaterialLibrary)))))))))
    (:then_8
      (if (Variables|/Game/Myriad/BP/BP_AudioSource.BP_AudioSource_C|GetEntityPulsing (Variables|Default|GetEntity))
        (Niagara|SetNiagaraVariable(Float) _niagaralightning "User.SpawnBeam2" 1.0)
        (Niagara|SetNiagaraVariable(Float) _niagaralightning "User.SpawnBeam1" 0.0)
        (else
          (Niagara|SetNiagaraVariable(Float) _niagaralightning "User.SpawnBeam2" 0.0)
          (Niagara|SetNiagaraVariable(Float) _niagaralightning "User.SpawnBeam1" 1.0))))
    (:then_9
      (Niagara|SetNiagaraVariable(Vector3) _niagaralightning "User.BeamEnd2" (Transformation|GetWorldLocation (Variables|/Script/Engine.Actor|GetRootComponent (Variables|Default|GetPlayer))))
      (Niagara|SetNiagaraVariable(Vector3) _niagaralightning "User.BeamEnd1" (Math|Random|RandomPointinBoundingBox "0, 0, 0" "800.000000,800.000000,-800.000000"))
      (Niagara|SetNiagaraVariable(Float) _niagaralightning "User.EmissiveMultiplier" 1.0))))

(fn ConstructionScript
  (bind _returnvalue (Rendering|Material|CreateDynamicMaterialInstance (Variables|Default|GetTerrain) 0 (Variables|Default|GetSourceMatTerrain) "None" :!class /Script/Engine.PrimitiveComponent))
  (bind _output_get (Variables|Default|SetDynamicMatTerrain _returnvalue)))